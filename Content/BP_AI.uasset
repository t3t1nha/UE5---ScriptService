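; BP_AI is an AI pawn that walks through BP_Waypoint actors placed in its Waypoints list.
; FollowWaypoint loops AIMoveTo on the current index, printing each reached waypoint's name, then destroying and removing it until the list empties.
; OnSpawnWaypoint refreshes the list from all level waypoints and restarts movement.
; OnClearWaypoint refreshes it and sets a flag that skips destruction when the pending move succeeds.
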(event Custom|Follow%20Waypoint
  (bind _waypoints (Variables|Default|GetWaypoints))
  (bind _current_waypoint (Variables|Default|GetCurrent%20Waypoint))
  (bind _waypoints_2 (Variables|Default|GetWaypoints))
  (bind _output (Utilities|Array|Get(acopy) _waypoints _current_waypoint))
  (if (Variables|Default|GetDid%20Clear%20waypoint?)
    (Variables|Default|SetDid%20Clear%20waypoint? false))
  (if (not (Variables|Default|GetIs%20at%20last%20waypoint?))
    (if (Utilities|Array|IsNotEmpty _waypoints)
      (AI|AIMoveTo self "0, 0, 0" _output 5.0 false
        (:OnSuccess
          (CallFunction|GottoWaypoint _output)
          (if (Variables|Default|GetDid%20Clear%20waypoint?)
            (Variables|Default|SetDid%20Clear%20waypoint? false)
            (else
              (Actor|DestroyActor _output)
              (Utilities|Array|RemoveIndex _waypoints_2 (Variables|Default|GetCurrent%20Waypoint))
              (Variables|Default|SetIs%20at%20last%20waypoint? (>= 0 (Utilities|Array|Length _waypoints_2)))
              (Utilities|FlowControl|Delay 0.2)))
          (CallFunction|FollowWaypoint))))))

(event EventBeginPlay
  (CallFunction|FollowWaypoint))

(event EventOnClearWaypoint
  (CallFunction|GetWaypoints)
  (Variables|Default|SetDid%20Clear%20waypoint? true))

(event EventOnSpawnWaypoint
  (CallFunction|GetWaypoints)
  (CallFunction|FollowWaypoint))

(fn ConstructionScript)

(fn GottoWaypoint
  (params (Waypoint :type BP%20Waypoint%20Object%20Reference))
  (Development|PrintString (Utilities|GetDisplayName Waypoint)))

(fn GetWaypoints
  (bind _outactors (Actor|GetAllActorsOfClass "/Game/BP_Waypoint.BP_Waypoint_C"))
  (Variables|Default|SetWaypoints _outactors)
  (Variables|Default|SetIs%20at%20last%20waypoint? false))