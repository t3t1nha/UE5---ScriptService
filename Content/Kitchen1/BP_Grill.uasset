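; BP_Grill is a kitchen grill meant to turn items into cooked outputs using recipes from a data table.
; BeginPlay caches the player character and loads the table rows into a recipe array.
; Unwired logic would match an overlapping BP_Item's class, wait the recipe delay, spawn the output and update the player's held item.
; The trigger's overlap event currently does nothing, and the Timer function is an unfinished stub.
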(event OnComponentBeginOverlap(GrillTrigger)
  (params (OverlappedComponent :type Primitive%20Component%20Object%20Reference) (OtherActor :type Actor%20Object%20Reference) (OtherComp :type Primitive%20Component%20Object%20Reference) (OtherBodyIndex :type Integer) (bFromSweep :type Boolean) (SweepResult :type Hit%20Result%20Structure%20%28by%20ref%29)))

(event EventBeginPlay
  ;[0.02609 0.15 0 0.5] Grab References
  (bind _returnvalue (Actor|GetActorOfClass "/Game/Characters/Blueprints/Player/BP_FirstPersonCharacter.BP_FirstPersonCharacter_C"))
  (Variables|Default|SetPlayerRef _returnvalue)
  (bind _recipearray (CallFunction|GetAllRecipesfromDataTable (Variables|Default|GetRecipesDataTable)))
  (Variables|Default|SetRecipesArray _recipearray))

(fn ConstructionScript)

(fn GetAllRecipesfromDataTable
  (params (Data%20Table :type Data%20Table%20Object%20Reference))
  (bind _recipearray (LocalVariables|GetRecipeArray))
  (bind _outrownames (DataTable|GetDataTableRowNames Data%20Table))
  (for _array_element _outrownames
    (bind _returnvalue (Utilities|GetDataTableRow Data%20Table _array_element)
      (:then
        (Utilities|Array|Add _recipearray (Utilities|Struct|MakeFallbackStruct (.Input (Utilities|Struct|BreakFallbackStruct _returnvalue)) (.Output (Utilities|Struct|BreakFallbackStruct _returnvalue)) (.Delay (Utilities|Struct|BreakFallbackStruct _returnvalue)))))
      (:RowNotFound
        (Development|PrintString "Row Not Found"))))
  (return _recipearray))

(fn Timer
  (params (Time :type Float%20%28double-precision%29))
  (LocalVariables|SetLocalTimer Time)
  (while false
    _))