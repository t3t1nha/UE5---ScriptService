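; Restaurant table actor that tracks which dishes are possible and shows an order indicator.
; On BeginPlay it binds to the game instance's item-unlocked event, which looks up the unlocked recipe names in a data table and stores their output item subclasses as PossibleDishes.
; Each tick it rotates the order indicator component to face the player camera.
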(event Custom|OnItemUnlocked
  (bind _recipeclasses (CallFunction|GetRecipeClass (Variables|/Game/EvergreenKit/Demo/Maps/BP_GameInstance.BP_GameInstance_C|GetUnlockedRecipeNameCopy (Variables|Default|GetGameInstanceRef))))
  (Variables|Default|SetPossibleDishes _recipeclasses))

(event EventBeginPlay
  (bind _returnvalue (Game|GetGameInstance))
  (bind _asbp_game_instance (Utilities|Casting|CastToBP_GameInstance _returnvalue))
  (EventDispatchers|BindEventtoOnItemUnlocked _asbp_game_instance (delegate Custom|OnItemUnlocked))
  (Variables|Default|SetGameInstanceRef _asbp_game_instance))

(event EventTick
  (params (DeltaSeconds :type Float%20%28single-precision%29))
  (bind _orderindicatorcomponent (Variables|Default|GetOrderIndicatorComponent))
  (Transformation|SetWorldRotation _orderindicatorcomponent (Math|Rotator|FindLookatRotation (Transformation|GetWorldLocation _orderindicatorcomponent) (Transformation|GetWorldLocation (Variables|/Script/Engine.PlayerCameraManager|GetTransformComponent (Game|GetPlayerCameraManager 0)))) false false))

(fn ConstructionScript)

(fn GetRecipeClass
  (params (RowNames :type Array%20of%20Names))
  (for _array_element RowNames
    (bind _returnvalue (Utilities|GetDataTableRow "/Game/Cooking/Data/NewDataTable.NewDataTable" _array_element)
      (:then
        (Utilities|Array|Add (LocalVariables|GetRecipeClasses) (.outputitemsubclass _returnvalue)))))
  (return (LocalVariables|GetRecipeClasses)))