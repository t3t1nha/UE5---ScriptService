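; BP_Compiler runs the logic blocks placed in the player's robot UI as commands for the AI.
; On BeginPlay it caches references to the BP_AI and BP_FirstPersonCharacter actors.
; OnRun loops over the UI's placed widgets and switches on block type, with "Go to" calling the AI's GotToWaypoint.
; Each command fires directly within the loop, with debug prints for progress.
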(event Custom|OnRun
  (for _array_element (Variables|/Game/Logic_Blocks/WBP_RobotControl.WBP_RobotControl_C|GetPlacedWidgets (Variables|/Game/Characters/Blueprints/Player/BP_FirstPersonCharacter.BP_FirstPersonCharacter_C|GetR_robotUI (Variables|Refs|GetPlayer_Ref)))
    (switch Utilities|FlowControl|Switch|SwitchonE_BlockTypes (.blocktype _array_element)
      (:NewEnumerator0
        (Development|PrintString "Go_To")
        (Default|GottoWaypoint (Variables|Refs|GetAI_Ref)))))
  (Development|PrintString "Done"))

(event EventBeginPlay
  (bind _returnvalue (Actor|GetActorOfClass "/Game/Characters/Blueprints/BP_AI.BP_AI_C"))
  (Variables|Refs|SetAI_Ref _returnvalue)
  (bind _returnvalue_2 (Actor|GetActorOfClass "/Game/Characters/Blueprints/Player/BP_FirstPersonCharacter.BP_FirstPersonCharacter_C"))
  (Variables|Refs|SetPlayer_Ref _returnvalue_2))

(fn ConstructionScript)