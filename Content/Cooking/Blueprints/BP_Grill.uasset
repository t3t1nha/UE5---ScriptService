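; BP_Grill is a cooking grill that shows a world-space progress widget while cooking runs.
; BeginPlay caches and collapses the WBP_CookingProgress widget, and Tick turns it toward the player camera while visible.
; OnStartCooking shows the widget and starts a looping timer that feeds GetCookingProgress into it.
; OnFinishCooking sets progress to full and collapses the widget, without clearing the timer.
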(event Custom|PushProgressToWidget
  (Class|CookingProgressWidget|UpdateProgress (Variables|Default|GetCookingProgress) (Class|ApparatusActor|GetCookingProgress)))

(event EventBeginPlay
  (bind _aswbp_cooking_progresswidget (Utilities|Casting|CastToWBP_CookingProgresswidget (UserInterface|GetWidget (Variables|Default|GetWidget))))
  (bind _output_get (Variables|Default|SetCookingProgress _aswbp_cooking_progresswidget))
  (Widget|SetVisibility _output_get "Collapsed")
  (Variables|Default|SetPlayerCameraManager (Game|GetPlayerCameraManager 0)))

(event EventOnStartCooking
  (Widget|SetVisibility (Variables|Default|GetCookingProgress) "Visible")
  (Utilities|Time|ClearandInvalidateTimerbyHandle (Variables|Default|GetProgressUpdate))
  (bind _returnvalue (Utilities|Time|SetTimerbyEvent (delegate Custom|PushProgressToWidget) 0.05 true))
  (Variables|Default|SetProgressUpdate _returnvalue))

(event EventOnFinishCooking
  (bind _cookingprogress (Variables|Default|GetCookingProgress))
  (Class|CookingProgressWidget|UpdateProgress _cookingprogress 1.0)
  (Widget|SetVisibility _cookingprogress "Collapsed"))

(event EventTick
  (params (DeltaSeconds :type Float%20%28single-precision%29))
  (if (Widget|IsVisible (Variables|Default|GetCookingProgress))
    (Transformation|SetWorldRotation (Variables|Default|GetWidget) (Math|Rotator|FindLookatRotation (Transformation|GetWorldLocation (Variables|Default|GetWidget)) (Camera|GetCameraLocation (Variables|Default|GetPlayerCameraManager))) false false)))

(fn ConstructionScript)