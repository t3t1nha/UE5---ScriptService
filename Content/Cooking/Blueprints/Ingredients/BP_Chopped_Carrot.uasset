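; BP_Chopped_Carrot is a cooking ingredient Blueprint for chopped carrot that spawns an actor when interacted with.
; Interact spawns the actor at its own transform, shifted by an Offset, then increments CurUses.
; The spawn runs only when MaxUses is less than CurUses, which appears inverted for a use limit.
; BeginPlay, overlap, Tick and the construction script are empty.
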(event EventBeginPlay)

(event Collision|EventActorBeginOverlap
  (params (OtherActor :type Actor%20Object%20Reference)))

(event EventTick
  (params (DeltaSeconds :type Float%20%28single-precision%29)))

(event EventInteract
  (bind _returnvalue (Transformation|GetActorTransform))
  (if (< (Variables|Default|GetMax_Uses) (Variables|Default|GetCur_Uses))
    (Game|SpawnActorfromClass "/Game/Cooking/Blueprints/Ingredients/BP_Carrot_Slice.BP_Carrot_Slice_C" (Math|Transform|MakeTransform (+ (.location _returnvalue) (Variables|Default|GetOffset)) (.rotation _returnvalue) (.scale _returnvalue)) "Undefined" "MultiplyWithRoot" 0 0)
    (Math|Integer|IncrementInt (Variables|Default|GetCur_Uses))))

(fn ConstructionScript)